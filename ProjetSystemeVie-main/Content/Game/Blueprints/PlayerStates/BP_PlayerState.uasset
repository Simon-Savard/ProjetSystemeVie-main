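; Player state that keeps player health persistent through BP_GameInstance and triggers respawn on death.
; On BeginPlay it restores health from the game instance, or resets the health component the first time and flags it initialized.
; Health changes are written back to the game instance, with current and max values crossed between the two save functions.
; Death asks BP_ThirdPersonGameMode to respawn player controller 0.
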(event OnHealthChanged(AC_Health_RG)
  (params (CurrentHealth :type Float%20%28double-precision%29) (MaxHealth :type Float%20%28double-precision%29))
  (CallFunction|SaveMaxHealth CurrentHealth)
  (CallFunction|SaveCurrentHealth MaxHealth))

(event OnDeath(AC_Health_RG)
  (bind _asbp_third_person_game_mode (Utilities|Casting|CastToBP_ThirdPersonGameMode (Game|GetGameMode)))
  (Default|StartRespawn _asbp_third_person_game_mode (Game|GetPlayerController 0)))

(event EventBeginPlay
  (bind _asbp_game_instance (Utilities|Casting|CastToBP_GameInstance (Game|GetGameInstance)))
  (bind _output_get (Variables|Default|SetGameInstanceRef _asbp_game_instance))
  (if (Variables|/Game/Game/Blueprints/BP_GameInstance.BP_GameInstance_C|GetHealthInitializedGI _output_get)
    (CallFunction|LoadHealthfromGI)
    (else
      (Default|ResetHealth (Variables|Default|GetAC_Health_RG))
      (Variables|/Game/Game/Blueprints/BP_GameInstance.BP_GameInstance_C|SetHealthInitializedGI (Variables|Default|GetGameInstanceRef) true))))

(fn ConstructionScript)

(fn SaveMaxHealth
  (params (NewMaxHealth :type Float%20%28double-precision%29))
  (Variables|/Game/Game/Blueprints/BP_GameInstance.BP_GameInstance_C|SetMaxHealthGI (Variables|Default|GetGameInstanceRef) NewMaxHealth))

(fn SaveCurrentHealth
  (params (NewCurrentHealth :type Float%20%28double-precision%29))
  (Variables|/Game/Game/Blueprints/BP_GameInstance.BP_GameInstance_C|SetCurrentHealthGI (Variables|Default|GetGameInstanceRef) NewCurrentHealth))

(fn LoadHealthfromGI
  (bind _ac_health_rg (Variables|Default|GetAC_Health_RG))
  (bind _output_get (Variables|/Game/Game/Blueprints/Components/AC_Health_RG.AC_Health_RG_C|SetMaxHealth _ac_health_rg (Variables|/Game/Game/Blueprints/BP_GameInstance.BP_GameInstance_C|GetMaxHealthGI (Variables|Default|GetGameInstanceRef))))
  (bind _output_get_2 (Variables|/Game/Game/Blueprints/Components/AC_Health_RG.AC_Health_RG_C|SetCurrentHealth _ac_health_rg (Variables|/Game/Game/Blueprints/BP_GameInstance.BP_GameInstance_C|GetCurrentHealthGI (Variables|Default|GetGameInstanceRef))))
  (Default|CallOnHealthChanged (Variables|Default|GetAC_Health_RG) _output_get_2 _output_get))