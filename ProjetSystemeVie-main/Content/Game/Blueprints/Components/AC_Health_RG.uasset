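; AC_Health_RG is a health component that tracks current health and a death state for its owner.
; Damage and heal events are ignored once dead, while a reset clears the death state and restores full health.
; All three route through UpdateHealthAndNotify, which clamps the value between zero and max, prints it, fires OnHealthChanged and fires OnDeath at zero.
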(event EventTakeDamage
  (params (DmgAmount :type Float%20%28double-precision%29))
  (if (not (Variables|Default|GetIsDead))
    (CallFunction|UpdateHealthandNotify (- (Variables|Default|GetCurrentHealth) DmgAmount))))

(event EventGainHealth
  (params (HealthAmount :type Float%20%28double-precision%29))
  (if (not (Variables|Default|GetIsDead))
    (CallFunction|UpdateHealthandNotify (+ (Variables|Default|GetCurrentHealth) HealthAmount))))

(event EventResetHealth
  (Variables|Default|SetIsDead false)
  (CallFunction|UpdateHealthandNotify (Variables|Default|GetMaxHealth)))

(fn UpdateHealthandNotify
  (params (NewHealthValue :type Float%20%28double-precision%29))
  (bind _maxhealth (Variables|Default|GetMaxHealth))
  (bind _returnvalue (Math|Float|Clamp(Float) NewHealthValue 0.0 _maxhealth))
  ;[0.15 0.15 0.15 0.5] MAJ var Healths dans AC_Health
  (Development|PrintString (Utilities|String|ToString(Float) _returnvalue))
  (bind _output_get (Variables|Default|SetCurrentHealth _returnvalue))
  (Default|CallOnHealthChanged _output_get (Variables|Default|GetMaxHealth))
  (if (<= (Variables|Default|GetCurrentHealth) 0.0)
    (Variables|Default|SetIsDead true)
    (Default|CallOnDeath)
    (else
      (Variables|Default|SetIsDead false))))